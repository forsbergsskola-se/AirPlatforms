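; CharacterAir is a player character with camera-relative movement, jumping, and a slow-motion aimed launch.
; Holding PrimaryAction dilates global time and shows a post-process effect, and releasing restores both and launches the character along the camera's forward vector, overriding its velocity.
; Tick steps the camera field of view, widening it quickly during slow motion and easing it back gradually afterwards.
; A CurrentCharges variable exists but is unused.
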(event EventBeginPlay)

(event Collision|EventActorBeginOverlap
  (params (OtherActor :type Actor%20Object%20Reference)))

(event EventTick
  (params (DeltaSeconds :type Float%20%28single-precision%29))
  (Camera|SetFieldOfView (Variables|Default|GetCamera) (Variables|Default|GetCurrent%20Field%20of%20view))
  (if (Variables|Default|GetPaused)
    (if (>= 1e+02 (Variables|Default|GetCurrent%20Field%20of%20view))
      (Variables|Default|SetCurrent%20Field%20of%20view (+ (Variables|Default|GetCurrent%20Field%20of%20view) 1.0)))
    (elif (>= (Variables|Default|GetCurrent%20Field%20of%20view) 95.0)
      (Variables|Default|SetCurrent%20Field%20of%20view (+ (Variables|Default|GetCurrent%20Field%20of%20view) -0.1)))))

(event Input|ActionEvents|InputActionJump
  (params (Key :type Key%20Structure :default "None"))
  (:Pressed
    (Character|Jump)))

(event Input|ActionEvents|InputActionPrimaryAction
  (params (Key :type Key%20Structure :default "None"))
  (bind _postprocess (Variables|Default|GetPostProcess))
  (:Pressed
    (Utilities|Time|SetGlobalTimeDilation 0.2)
    (Variables|Default|SetPaused true)
    (Rendering|SetVisibility _postprocess true true))
  (:Released
    (Utilities|Time|SetGlobalTimeDilation 1.0)
    (Character|LaunchCharacter (* (Math|Vector|GetForwardVector (Variables|Default|GetCamera)) "1500.000000,1500.000000,1500.000000") true true)
    (Variables|Default|SetPaused false)
    (Rendering|SetVisibility _postprocess false false)))

(event Input|AxisEvents|InputAxisLookUp/DownGamepad
  (params (AxisValue :type Float%20%28single-precision%29))
  (Pawn|Input|AddControllerPitchInput (* AxisValue (Variables|Default|GetMouse%20sensitivity))))

(event Input|AxisEvents|InputAxisLookUp/DownMouse
  (params (AxisValue :type Float%20%28single-precision%29))
  (Pawn|Input|AddControllerPitchInput (* AxisValue (Variables|Default|GetMouse%20sensitivity))))

(event Input|AxisEvents|InputAxisTurnRight/LeftGamepad
  (params (AxisValue :type Float%20%28single-precision%29))
  (Pawn|Input|AddControllerYawInput (* AxisValue (Variables|Default|GetMouse%20sensitivity))))

(event Input|AxisEvents|InputAxisTurnRight/LeftMouse
  (params (AxisValue :type Float%20%28single-precision%29))
  (Pawn|Input|AddControllerYawInput (* AxisValue (Variables|Default|GetMouse%20sensitivity))))

(event Input|AxisEvents|InputAxisMoveForward/Backward
  (params (AxisValue :type Float%20%28single-precision%29))
  (Pawn|Input|AddMovementInput (Math|Vector|GetForwardVector (Variables|Default|GetCamera)) AxisValue false))

(event Input|AxisEvents|InputAxisMoveRight/Left
  (params (AxisValue :type Float%20%28single-precision%29))
  (Pawn|Input|AddMovementInput (Math|Vector|GetRightVector (Variables|Default|GetCamera)) AxisValue false))

(fn ConstructionScript
  (Rendering|SetVisibility (Variables|Default|GetPostProcess) false false))
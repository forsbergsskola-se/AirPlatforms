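; Timed trap actor that toggles a kill plane on and off and restarts the level when the player's CharacterAir touches it.
; A looping timer started at BeginPlay flips the plane's visibility and the Box's overlap event generation together, tracked by two booleans.
; An overlap with CharacterAir while the trap is active reloads FirstPersonMap by name.
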(event Custom|Flip%20Killplane
  (Rendering|SetVisibility (Variables|Default|GetKillPlane) (not (Variables|Default|GetPlaneVis)) false)
  (Variables|/Script/Engine.PrimitiveComponent|SetbGenerateOverlapEvents (Variables|Default|GetBox) (not (Variables|Default|GetPlaneCol)))
  (Variables|Default|SetPlaneCol (not (Variables|Default|GetPlaneCol)))
  (Variables|Default|SetPlaneVis (not (Variables|Default|GetPlaneVis))))

(event EventBeginPlay
  (Utilities|Time|SetTimerbyEvent (delegate Custom|Flip%20Killplane) (Variables|Default|GetTimer) true))

(event Collision|EventActorBeginOverlap
  (params (OtherActor :type Actor%20Object%20Reference))
  (Utilities|Casting|CastToCharacterAir OtherActor)
  (Game|OpenLevel(byName) "FirstPersonMap"))

(fn ConstructionScript)